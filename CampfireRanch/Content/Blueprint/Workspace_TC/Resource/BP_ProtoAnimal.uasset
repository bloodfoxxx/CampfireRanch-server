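; Prototype farm animal that spawns egg and milk collectibles, using BP_Collectibles with a swapped mesh at its spawn point.
; A fast Tick spawns milk when the Rancher has entered InteractionBox and is interacting, then sets Bite.
; While Bite is true, the head jitters randomly and the egg DoOnce resets.
; Otherwise, that DoOnce drops one egg automatically when no interaction occurs; nothing here clears Bite.
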(event `self.ReceiveBeginPlay`
  ;[1 1 1] Setup
  (`self.SetActorTickInterval` 0.01)
  (bind _asbp_rancher (cast `/Game/Blueprint/Workspace_TC/Character/BP_Rancher` (`GameplayStatics.GetPlayerPawn` 0)))
  (set `self.As BP Rancher` _asbp_rancher))

(event `self.InteractionBox.OnComponentBeginOverlap`
  (params (OverlappedComponent :type "PrimitiveComponent Object Reference") (OtherActor :type "Actor Object Reference") (OtherComp :type "PrimitiveComponent Object Reference") (OtherBodyIndex :type Integer) (bFromSweep :type Boolean) (SweepResult :type "HitResult Structure (by ref)"))
  ;[1 1 1] Set "Player is close to me"
  (if (== OtherActor (`self.As BP Rancher`))
    (set `self.Player Interaction` true)))

(event `self.ReceiveTick`
  (params (DeltaSeconds :type "Float (single-precision)"))
  (bind (_returnvalue_location _returnvalue_rotation) (`KismetMathLibrary.BreakTransform` (`SceneComponent.K2_GetComponentToWorld` (`self.SpawnCollsion`))))
  (bind (_returnvalue_location_2 _returnvalue_rotation_2) (`KismetMathLibrary.BreakTransform` (`SceneComponent.K2_GetComponentToWorld` (`self.SpawnCollsion`))))
  ;[1 1 1] Do I need to wait to produce goddies?
  (if (`self.Bite`)
    ;[1 1 1] My animation (indicating romaing)
    (`SceneComponent.K2_SetRelativeRotation` (`self.Head`) (`KismetMathLibrary.MakeRotator` (`KismetMathLibrary.RandomFloatInRange` -40.0 -20.0)) false false)
    (goto _label_2 :!via `Reset`)
    (else
      ;[1 1 1] Is the player close to me?
      (if (`self.Player Interaction`)
        (bind _asbp_rancher (cast `/Game/Blueprint/Workspace_TC/Character/BP_Rancher` (`GameplayStatics.GetPlayerPawn` 0)))
        ;[1 1 1] Is the player pressing interaction key?
        (if (`/Game/Blueprint/Workspace_TC/Character/BP_Rancher.Is Interacting` _asbp_rancher)
          ;[1 1 1] Manual action: spawn milk
          (`/Engine/EditorBlueprintResources/StandardMacros.DoOnce` false :!label _label
            (:`Completed`
              (bind _returnvalue (`|SpawnActorFromClass` "/Game/Blueprint/Workspace_TC/Resource/BP_Collectibles.BP_Collectibles_C" (`KismetMathLibrary.MakeTransform` _returnvalue_location _returnvalue_rotation (0.5 0.5 0.5)) "Undefined" "OverrideRootScale" null null))
              (`StaticMeshComponent.SetStaticMesh` (`/Game/Blueprint/Workspace_TC/Resource/BP_Collectibles.Collectible Mesh` _returnvalue) (`self.Milk`))
              (set `self.Bite` true)
              (set `self.Player Interaction` false)
              (goto _label :!via `Reset`)))
          (else
            _)))
      ;[1 1 1] Automatic action: spawn egg
      (`/Engine/EditorBlueprintResources/StandardMacros.DoOnce` false :!label _label_2
        (:`Completed`
          (bind _returnvalue_2 (`|SpawnActorFromClass` "/Game/Blueprint/Workspace_TC/Resource/BP_Collectibles.BP_Collectibles_C" (`KismetMathLibrary.MakeTransform` _returnvalue_location_2 _returnvalue_rotation_2 (0.5 0.5 0.5)) "Undefined" "OverrideRootScale" null null))
          (`StaticMeshComponent.SetStaticMesh` (`/Game/Blueprint/Workspace_TC/Resource/BP_Collectibles.Collectible Mesh` _returnvalue_2) (`self.Egg`)))))))

(fn `UserConstructionScript`)