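; Player character for the rancher, handling movement, jumping, interaction and pause input.
; On BeginPlay it caches the game mode and instance, adds a temporary testing widget, teleports to the transform stored in the game instance, then sets PlayerStart.
; PlayerStart gates control-rotation-relative movement, jumping and the IsInteracting flag set while the interact input is held.
; The pause input uses a FlipFlop to toggle the testing pause widget, game pause, cursor and input mode.
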(event `self.ReceiveBeginPlay`
  ;[1 1 1] Setup
  (bind _asbp_cr_game_mode (cast `/Game/Blueprint/Workspace_TC/World/BP_CR_GameMode` (`GameplayStatics.GetGameMode`)))
  (set `self.As BP CR Game Mode` _asbp_cr_game_mode)
  (bind _asbp_cr_game_instance (cast `/Game/Blueprint/Workspace_TC/World/BP_CR_GameInstance` (`GameplayStatics.GetGameInstance`)))
  (bind _output_get (set `self.As BP CR Game Instance` _asbp_cr_game_instance))
  ;[1 1 1] Add Testing Widget, TEMPORARY
  (bind _returnvalue (`|CreateWidget` "/Game/Blueprint/Workspace_TC/UI/BP_TestingWidget.BP_TestingWidget_C"))
  (`UserWidget.AddToViewport` _returnvalue 0)
  ;[1 1 1] Load Player location
  (`self.K2_SetActorTransform` (`/Game/Blueprint/Workspace_TC/World/BP_CR_GameInstance.Instance Player Transform` _output_get) false true)
  ;[1 1 1] Start actions
  (set `self.Player Start` true))

(event `InputAxis|Vertical Movement`
  (params (AxisValue :type "Float (single-precision)"))
  (bind (_returnvalue_roll _returnvalue_pitch _returnvalue_yaw) (`KismetMathLibrary.BreakRotator` (`self.GetControlRotation`)))
  ;[1 1 1] Movement
  (if (`self.Player Start`)
    (`self.AddMovementInput` (`KismetMathLibrary.GetForwardVector` (`KismetMathLibrary.MakeRotator` 0.0 0.0 _returnvalue_yaw)) AxisValue)))

(event `InputAction|Pause Trigger`
  (params (Key :type "Key Structure"))
  (bind _returnvalue (`GameplayStatics.GetPlayerController` 0))
  (bind _returnvalue_2 (`GameplayStatics.GetPlayerController` 0))
  (:`Pressed`
    ;[1 1 1] Open Pause menu
    (`/Engine/EditorBlueprintResources/StandardMacros.FlipFlop`
      (:`A`
        (bind _returnvalue_3 (`|CreateWidget` "/Game/Blueprint/Workspace_TC/UI/BP_TestingPauseWidget.BP_TestingPauseWidget_C"))
        (`UserWidget.AddToViewport` _returnvalue_3 0)
        (`GameplayStatics.SetGamePaused` true)
        (`WidgetBlueprintLibrary.SetInputMode_GameAndUIEx` _returnvalue_2 null)
        (set `PlayerController.bShowMouseCursor` true _returnvalue_2))
      (:`B`
        (`Widget.RemoveFromParent` _returnvalue_3)
        (`WidgetBlueprintLibrary.SetInputMode_GameOnly` _returnvalue)
        (set `PlayerController.bShowMouseCursor` false _returnvalue)
        (`GameplayStatics.SetGamePaused` false)))))

(event `InputAxis|Horizontal Movement`
  (params (AxisValue :type "Float (single-precision)"))
  (bind (_returnvalue_roll _returnvalue_pitch _returnvalue_yaw) (`KismetMathLibrary.BreakRotator` (`self.GetControlRotation`)))
  ;[1 1 1] Movement
  (if (`self.Player Start`)
    (`self.AddMovementInput` (`KismetMathLibrary.GetRightVector` (`KismetMathLibrary.MakeRotator` _returnvalue_roll 0.0 _returnvalue_yaw)) AxisValue)))

(event `InputAction|Interaction Trigger`
  (params (Key :type "Key Structure"))
  (bind _player_start (`self.Player Start`))
  ;[1 1 1] Interacting
  (:`Pressed`
    (if _player_start
      (set `self.Is Interacting` true)))
  (:`Released`
    (if _player_start
      (set `self.Is Interacting` false))))

(event `InputAction|Jump Trigger`
  (params (Key :type "Key Structure"))
  (bind _player_start (`self.Player Start`))
  ;[1 1 1] Movement
  (:`Pressed`
    (if _player_start
      (`self.Jump`)))
  (:`Released`
    (if _player_start
      (`self.StopJumping`))))

(fn `UserConstructionScript`)