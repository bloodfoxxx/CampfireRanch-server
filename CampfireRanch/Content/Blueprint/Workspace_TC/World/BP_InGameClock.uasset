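; BP_InGameClock is the in-game clock, counting minutes, hours, days, seasons and years on a running total kept in the game instance.
; After a short delay on BeginPlay, it splits the saved InstanceTime into units, though the final split assigns the quotient to Minutes and remainder to Hours.
; A looping timer, scaled by TestingParameter, runs Clock to cascade rollovers and save the total.
; Clock never increments Years, even when seasons wrap.
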(event `self.ReceiveBeginPlay`
  ;[1 1 1] Basic Setup
  (`KismetSystemLibrary.Delay` 0.5)
  (bind _asbp_cr_game_instance (cast `/Game/Blueprint/Workspace_TC/World/BP_CR_GameInstance` (`GameplayStatics.GetGameInstance`)))
  (bind _output_get (set `self.As BP CR Game Instance` _asbp_cr_game_instance))
  (bind _output_get_2 (set `self.Total Time` (`/Game/Blueprint/Workspace_TC/World/BP_CR_GameInstance.Instance Time` _output_get)))
  (bind (_remainder _returnvalue) (`KismetMathLibrary.FMod` (`KismetMathLibrary.Conv_IntToDouble` _output_get_2) 172800.0))
  ;[1 1 1] Convert total time to current time in respective units
  (set `self.Years` (+ 1 _returnvalue))
  (bind (_remainder_2 _returnvalue_2) (`KismetMathLibrary.FMod` _remainder 43200.0))
  (set `self.Seasons` (+ 1 _returnvalue_2))
  (bind (_remainder_3 _returnvalue_3) (`KismetMathLibrary.FMod` _remainder_2 1440.0))
  (set `self.Days` (+ 1 _returnvalue_3))
  (bind (_remainder_4 _returnvalue_4) (`KismetMathLibrary.FMod` _remainder_3 60.0))
  (set `self.Hours` (`KismetMathLibrary.FTrunc` _remainder_4))
  (set `self.Minutes` _returnvalue_4)
  ;[1 1 1] Clock Function
  (`KismetSystemLibrary.K2_SetTimer` null "Clock" (/ 1.0 (`self.Testing Parameter`)) true))

(event `Clock`
  ;[1 1 1] In crease time unit every second
  (if (<= (`self.Minutes`) 59)
    (`/Engine/EditorBlueprintResources/StandardMacros.IncrementInt` (`self.Minutes`)
      (:`  `
        (`/Engine/EditorBlueprintResources/StandardMacros.IncrementInt` (`self.Total Time`)
          (:`  `
            (set `/Game/Blueprint/Workspace_TC/World/BP_CR_GameInstance.Instance Time` (`self.Total Time`) (`self.As BP CR Game Instance`))))))
    (elif (<= (`self.Hours`) 23)
      (set `self.Minutes` 0)
      (`/Engine/EditorBlueprintResources/StandardMacros.IncrementInt` (`self.Hours`)
        (:`  `
          (`/Engine/EditorBlueprintResources/StandardMacros.IncrementInt` (`self.Total Time`)
            (:`  `
              (set `/Game/Blueprint/Workspace_TC/World/BP_CR_GameInstance.Instance Time` (`self.Total Time`) (`self.As BP CR Game Instance`))))))
      (elif (<= (`self.Days`) 29)
        (set `self.Minutes` 0)
        (set `self.Hours` 0)
        (`/Engine/EditorBlueprintResources/StandardMacros.IncrementInt` (`self.Days`)
          (:`  `
            (`/Engine/EditorBlueprintResources/StandardMacros.IncrementInt` (`self.Total Time`)
              (:`  `
                (set `/Game/Blueprint/Workspace_TC/World/BP_CR_GameInstance.Instance Time` (`self.Total Time`) (`self.As BP CR Game Instance`))))))
        (elif (<= (`self.Seasons`) 3)
          (set `self.Minutes` 0)
          (set `self.Hours` 0)
          (set `self.Days` 1)
          (`/Engine/EditorBlueprintResources/StandardMacros.IncrementInt` (`self.Seasons`)
            (:`  `
              (`/Engine/EditorBlueprintResources/StandardMacros.IncrementInt` (`self.Total Time`)
                (:`  `
                  (set `/Game/Blueprint/Workspace_TC/World/BP_CR_GameInstance.Instance Time` (`self.Total Time`) (`self.As BP CR Game Instance`))))))
          (else
            (set `self.Minutes` 0)
            (set `self.Hours` 0)
            (set `self.Days` 1)
            (set `self.Seasons` 1)
            (`/Engine/EditorBlueprintResources/StandardMacros.IncrementInt` (`self.Total Time`)
              (:`  `
                (set `/Game/Blueprint/Workspace_TC/World/BP_CR_GameInstance.Instance Time` (`self.Total Time`) (`self.As BP CR Game Instance`))))))))))

(fn `UserConstructionScript`)